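; BP_Cube is the player cube in Cube Runner, which runs forward, steers sideways and scores by distance.
; A looping timer applies forward velocity-change impulses while the right/left axis input applies sideways ones, both gated by a movement flag.
; Hitting an obstacle-tagged actor stops that movement input and reloads the current level after a delay.
; Tick derives the score from world X, and BeginPlay adds the BP_Score widget to the viewport.
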(event `self.ReceiveTick`
  (params (DeltaSeconds :type "Float (single-precision)"))
  (bind _returnvalue_x (`KismetMathLibrary.BreakVector` (`SceneComponent.K2_GetComponentLocation` (`self.Cube`))))
  (set `self.Score` (`KismetMathLibrary.FTrunc` (/ _returnvalue_x 100.0))))

(event `self.ReceiveBeginPlay`
  (bind _returnvalue (`|CreateWidget` "/Game/Cube_Runner/Widgets/BP_Score.BP_Score_C"))
  (`UserWidget.AddToViewport` _returnvalue 0)
  (`KismetSystemLibrary.K2_SetTimerDelegate` (delegate `Move_Cube`) 0.1 true))

(event `Move_Cube`
  (if (`self.CanMOve?`)
    (`PrimitiveComponent.AddImpulse` (`self.Cube`) (`KismetMathLibrary.MakeVector` (`self.Forward_Force`)) "None" true)))

(event `InputAxis|Move Right/Left`
  (params (AxisValue :type "Float (single-precision)"))
  (if (`self.CanMOve?`)
    (`PrimitiveComponent.AddImpulse` (`self.Cube`) (`KismetMathLibrary.MakeVector` 0.0 (* AxisValue (`self.Moveright?leftForce`))) "None" true)))

(event `RestartLevel`
  (`KismetSystemLibrary.Delay` (`self.RestartDelay`) :!label _label)
  (bind _returnvalue (`GameplayStatics.GetCurrentLevelName` true))
  (`GameplayStatics.OpenLevel` (`KismetStringLibrary.Conv_StringToName` _returnvalue)))

(event `self.Cube.OnComponentHit`
  (params (HitComponent :type "PrimitiveComponent Object Reference") (OtherActor :type "Actor Object Reference") (OtherComp :type "PrimitiveComponent Object Reference") (NormalImpulse :type "Vector Structure") (Hit :type "HitResult Structure (by ref)"))
  (if (`self.ActorHasTag` OtherActor "obstacle")
    (set `self.CanMOve?` false)
    (goto _label)))

(fn `UserConstructionScript`)